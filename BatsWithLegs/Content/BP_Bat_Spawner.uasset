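; Bat spawner that keeps adding BP_NPC_Bat actors at designated spawn points while their count is below MaxBatsAGT.
; Spawn runs from BeginPlay and re-calls itself after a short random delay.
; GetSpawnPoint loops until a random point is over 400 units from the player, but draws again for the returned location, which can therefore be nearer.
; The construction script adds an upward arrow for each spawn point.
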(event `self.ReceiveBeginPlay`
  (`self.Spawn`))

(event `Spawn`
  (bind _outactors (`GameplayStatics.GetAllActorsOfClass` "/Game/BP_NPC_Bat.BP_NPC_Bat_C"))
  (if (< (`KismetArrayLibrary.Array_Length` _outactors) (`self.Max Bats AGT`))
    (bind _location (`self.GetSpawnPoint`))
    (`|SpawnActorFromClass` "/Game/BP_NPC_Bat.BP_NPC_Bat_C" (`KismetMathLibrary.Conv_VectorToTransform` _location) "Undefined" "OverrideRootScale" null null))
  (`KismetSystemLibrary.Delay` (`KismetMathLibrary.RandomFloatInRange` 0.3 2.0))
  (`self.Spawn`))

(fn `GetSpawnPoint`
  (returns (Location :type "Vector Structure"))
  (bind _returnvalue (`self.K2_GetActorLocation` (`KismetArrayLibrary.Array_Random` (`self.Spawn Points`))))
  (while true
    (if (> (`KismetMathLibrary.Vector_Distance` _returnvalue (`self.K2_GetActorLocation` (`GameplayStatics.GetPlayerCharacter` 0))) 400.0)
      (return _returnvalue))))

(fn `UserConstructionScript`
  (for _array_element (`self.Spawn Points`)
    (`AddComponent|NODE_AddArrowComponent-0` :`RelativeTransform` (`KismetMathLibrary.MakeTransform` (`self.K2_GetActorLocation` _array_element) (`KismetMathLibrary.FindLookAtRotation` (`KismetMathLibrary.Vector_Zero`) (`KismetMathLibrary.Vector_Up`))))))