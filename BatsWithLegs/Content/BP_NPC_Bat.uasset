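; Flying bat enemy NPC that hovers at a random height offset and chases the player.
; A looping AIMoveTo re-targets the player's location after short delays, while Tick turns the mesh to face them.
; Overlapping the player while alive damages them and destroys the bat.
; At zero health it awards score, stops moving, gets knocked away from the player as a physics body, then despawns.
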(event `self.ReceiveBeginPlay`
  (`SceneComponent.K2_AddLocalOffset` (`self.StaticMesh`) (`KismetMathLibrary.MakeVector` 0.0 0.0 (`KismetMathLibrary.RandomFloatInRange` 100.0 250.0)) false false)
  (`self.MoveNPC`))

(event `MoveNPC`
  (bind _output_get (set `self.Random Location` (`self.K2_GetActorLocation` (`GameplayStatics.GetPlayerCharacter` 0))))
  (`|AIMoveTo` self _output_get null
    (:`OnSuccess`
      (`KismetSystemLibrary.Delay` 0.7))
    (:`OnFail`
      (`KismetSystemLibrary.Delay` 0.1)))
  (`self.MoveNPC`))

(event `Damage`
  (params (Damage :type "Float (double-precision)"))
  (bind _staticmesh (`self.StaticMesh`))
  (bind _output_get (set `self.health` (- (`self.health`) Damage)))
  (if (not (> _output_get 0.0))
    (`|ExecutionSequence`
      (:`then_0`
        (bind _asbp_first_person_character (cast `/Game/FirstPerson/Blueprints/BP_FirstPersonCharacter` (`GameplayStatics.GetPlayerCharacter` 0)))
        (`/Game/FirstPerson/Blueprints/BP_FirstPersonCharacter.IncreaseScore` _asbp_first_person_character))
      (:`then_1`
        (`NavMovementComponent.StopActiveMovement` (`self.FloatingPawnMovement`))
        (`ActorComponent.Deactivate` (`self.FloatingPawnMovement`))
        (`|ExecutionSequence`
          (:`then_0`
            (`PrimitiveComponent.SetSimulatePhysics` _staticmesh true)
            (`PrimitiveComponent.SetEnableGravity` _staticmesh true))
          (:`then_1`
            (`KismetSystemLibrary.Delay` 0.1)
            (`PrimitiveComponent.AddImpulse` (`self.StaticMesh`) (* (`KismetMathLibrary.Normal` (- (`self.K2_GetActorLocation` (`GameplayStatics.GetPlayerCharacter` 0)) (`self.K2_GetActorLocation`))) -500000.0) "None" false))
          (:`then_2`
            (`KismetSystemLibrary.Delay` 2.0)
            (`self.K2_DestroyActor`)))))))

(event `self.ReceiveActorBeginOverlap`
  (params (OtherActor :type "Actor Object Reference"))
  (bind _asbp_first_person_character (cast `/Game/FirstPerson/Blueprints/BP_FirstPersonCharacter` OtherActor))
  (if (> (`self.health`) 0.0)
    (`/Game/FirstPerson/Blueprints/BP_FirstPersonCharacter.TakeDamage` _asbp_first_person_character)
    (`self.K2_DestroyActor`)))

(event `self.ReceiveTick`
  (params (DeltaSeconds :type "Float (single-precision)"))
  (`SceneComponent.K2_SetRelativeRotation` (`self.StaticMesh`) (`KismetMathLibrary.Quat_Rotator` (`KismetMathLibrary.Quat_MakeFromEuler` (+ (`KismetMathLibrary.Quat_Euler` (`KismetMathLibrary.Conv_RotatorToQuaternion` (`KismetMathLibrary.FindLookAtRotation` (`self.K2_GetActorLocation`) (`self.K2_GetActorLocation` (`GameplayStatics.GetPlayerCharacter` 0))))) (0.0 0.0 -90.0)))) false false))

(fn `UserConstructionScript`)