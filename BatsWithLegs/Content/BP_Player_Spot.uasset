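; BP_Player_Spot is an actor that smoothly follows the first player's character from a set height above it.
; Each Tick, while that character is valid, it lerps its location toward the character's position plus a Height offset on Z.
; The lerp alpha is delta time times Smoothing, giving an eased trailing motion without sweeping; rotation is left untouched.
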(event `self.ReceiveTick`
  (params (DeltaSeconds :type "Float (single-precision)"))
  (bind _returnvalue (`GameplayStatics.GetPlayerCharacter` 0))
  (bind (_returnvalue_x _returnvalue_y _returnvalue_z) (`KismetMathLibrary.BreakVector` (`self.K2_GetActorLocation` _returnvalue)))
  (`/Engine/EditorBlueprintResources/StandardMacros.IsValid` _returnvalue
    (:`Is Valid`
      (`self.K2_SetActorLocation` (`KismetMathLibrary.VLerp` (`self.K2_GetActorLocation`) (`KismetMathLibrary.MakeVector` _returnvalue_x _returnvalue_y (+ _returnvalue_z (`self.Height`))) (* DeltaSeconds (`self.Smoothing`)))))))

(fn `UserConstructionScript`)